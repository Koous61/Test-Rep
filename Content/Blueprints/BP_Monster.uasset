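; BP_Monster is a monster Blueprint that takes damage against an integer Health value.
; AnyDamage subtracts the damage, truncates the result, passes it to SetHealth and prints whether that call succeeded.
; BeginPlay prints a debug message when CheckIsAndroid is false and IsServer is true.
; The custom event and construction script are empty.
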(event Custom|CustomEvent_0)

(event Game|Damage|EventAnyDamage
  (params (Damage :type Float%20%28single-precision%29) (DamageType :type Damage%20Type%20Object%20Reference) (InstigatedBy :type Controller%20Object%20Reference) (DamageCauser :type Actor%20Object%20Reference))
  (bind _returnvalue (Class|MonsterActorC|SetHealth (Math|Float|Truncate (- (Math|Conversions|ToFloat(Integer) (Variables|Default|GetHealth)) Damage))))
  (if _returnvalue
    (Development|PrintString "Damage apply")
    (else
      (Development|PrintString "Damage not apply"))))

(event EventBeginPlay
  (if (not (Class|MonsterActorC|CheckIsAndroid))
    (if (Networking|IsServer)
      (Development|PrintString "Server!!!!"))))

(fn ConstructionScript)